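; BP_Ethan is a physics-driven wandering AI actor that moves by flinging its Cube with impulses along navmesh paths.
; A looping timer picks a random navigable point around the world origin and calls the AI event dispatcher.
; The bound event finds a synchronous path, then applies distance-scaled velocity-change impulses toward each point, separated by random delays.
; Cube1 receives a random mass on BeginPlay.
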(event `self.ReceiveBeginPlay`
  (add `self.AI` (delegate `AI_Event`))
  (`KismetSystemLibrary.K2_SetTimer` null "SetRandomPos" 5.0 true)
  (`PrimitiveComponent.SetMassOverrideInKg` (`self.Cube1`) "None" (`KismetMathLibrary.RandomFloatInRange` 3.0 60.0) true))

(event `AI_Event`
  (bind _returnvalue (`SceneComponent.K2_GetComponentLocation` (`self.Cube`)))
  (bind _returnvalue_2 (`NavigationSystemV1.FindPathToLocationSynchronously` _returnvalue (`self.TargetPos`) (`AIBlueprintHelperLibrary.GetAIController` self) null))
  (bind _array_element (`/Engine/EditorBlueprintResources/ForLoopDelay.ForEachLoopWithDelay` (`NavigationPath.PathPoints` _returnvalue_2) :!label _label)
    (:`LoopBody`
      (`PrimitiveComponent.AddImpulse` (`self.Cube`) (* (`KismetMathLibrary.GetDirectionUnitVector` _returnvalue _array_element) (* (`self.Force`) (`KismetMathLibrary.Vector_Distance` _returnvalue _array_element))) "None" true)
      (`KismetSystemLibrary.Delay` (`KismetMathLibrary.RandomFloatInRange` 0.5 0.8))
      (goto _label :!via `Next`))))

(event `self.ReceiveTick`
  (params (DeltaSeconds :type "Float (single-precision)")))

(fn `SetRandomPos`
  (bind _randomlocation (`NavigationSystemV1.K2_GetRandomLocationInNavigableRadius` (`KismetMathLibrary.MakeVector` 0.0) 5000.0 null null))
  (set `self.TargetPos` _randomlocation)
  (`self.AI`))

(fn `UserConstructionScript`)